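; BP_SaveManager is an actor that saves and loads audio options and scores in separate slots, both using BP_AuroraSaveGame.
; On BeginPlay it applies saved volumes to BP_AudioManager, then loads scores into AuroraGameInstance unless its GameLoaded flag is already set.
; Tick polls ShouldSave flags on the game instance and audio manager, writing the matching slot from a fresh save object and clearing the flag.
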(event EventBeginPlay
  (CallFunction|LoadGame true)
  (bind _asaurora_game_instance (Utilities|Casting|CastToAuroraGameInstance (Game|GetGameInstance)))
  (if (not (Class|AuroraGameInstance|GameLoaded _asaurora_game_instance))
    (CallFunction|LoadGame false)
    (Class|AuroraGameInstance|SetGameLoaded _asaurora_game_instance true)))

(event Collision|EventActorBeginOverlap
  (params (OtherActor :type Actor%20Object%20Reference)))

(event EventTick
  (params (DeltaSeconds :type Float%20%28single-precision%29))
  (Utilities|FlowControl|Sequence
    (:then_0
      (bind _asaurora_game_instance (Utilities|Casting|CastToAuroraGameInstance (Game|GetGameInstance)))
      (if (Class|AuroraGameInstance|ShouldSave _asaurora_game_instance)
        (CallFunction|SaveGame false)
        (Class|AuroraGameInstance|SetShouldSave _asaurora_game_instance false)))
    (:then_1
      (bind _returnvalue (Actor|GetActorOfClass "/Game/Mechanics/AudioManager/BP_AudioManager.BP_AudioManager_C"))
      (if (Class|AudioManager|ShouldSave _returnvalue)
        (CallFunction|SaveGame true)
        (Class|AudioManager|SetShouldSave _returnvalue false)))))

(fn ConstructionScript)

(fn LoadGame
  (params (OnlyLoadOptions :type Boolean))
  (if OnlyLoadOptions
    (bind _returnvalue (SaveGame|LoadGamefromSlot "Options"))
    (bind _asbp_aurora_save_game (Utilities|Casting|CastToBP_AuroraSaveGame _returnvalue))
    (bind _returnvalue_2 (Actor|GetActorOfClass "/Game/Mechanics/AudioManager/BP_AudioManager.BP_AudioManager_C"))
    (Utilities|FlowControl|Sequence
      (:then_0
        (Class|AudioManager|SetVolume _returnvalue_2 "Master" (Variables|/Game/GameModes/Saving/BP_AuroraSaveGame.BP_AuroraSaveGame_C|GetMasterVolume _asbp_aurora_save_game)))
      (:then_1
        (Class|AudioManager|SetVolume _returnvalue_2 "Music" (Variables|/Game/GameModes/Saving/BP_AuroraSaveGame.BP_AuroraSaveGame_C|GetMusicVolume _asbp_aurora_save_game)))
      (:then_2
        (Class|AudioManager|SetVolume _returnvalue_2 "SFX" (Variables|/Game/GameModes/Saving/BP_AuroraSaveGame.BP_AuroraSaveGame_C|GetSFXVolume _asbp_aurora_save_game))))
    (else
      (bind _returnvalue_3 (SaveGame|LoadGamefromSlot "Scores"))
      (bind _asbp_aurora_save_game_2 (Utilities|Casting|CastToBP_AuroraSaveGame _returnvalue_3))
      (bind _asaurora_game_instance (Utilities|Casting|CastToAuroraGameInstance (Game|GetGameInstance)))
      (Class|AuroraGameInstance|SetScores _asaurora_game_instance (Variables|/Game/GameModes/Saving/BP_AuroraSaveGame.BP_AuroraSaveGame_C|GetScores _asbp_aurora_save_game_2)))))

(fn SaveGame
  (params (OnlySaveOptions :type Boolean))
  (if OnlySaveOptions
    (bind _returnvalue (SaveGame|CreateSaveGameObject "/Game/GameModes/Saving/BP_AuroraSaveGame.BP_AuroraSaveGame_C"))
    (bind _returnvalue_2 (Actor|GetActorOfClass "/Game/Mechanics/AudioManager/BP_AudioManager.BP_AudioManager_C"))
    (Variables|/Game/GameModes/Saving/BP_AuroraSaveGame.BP_AuroraSaveGame_C|SetMasterVolume _returnvalue (Class|AudioManager|GetMasterVolume _returnvalue_2))
    (Variables|/Game/GameModes/Saving/BP_AuroraSaveGame.BP_AuroraSaveGame_C|SetMusicVolume _returnvalue (Class|AudioManager|GetMusicVolume _returnvalue_2))
    (Variables|/Game/GameModes/Saving/BP_AuroraSaveGame.BP_AuroraSaveGame_C|SetSFXVolume _returnvalue (Class|AudioManager|GetSFXVolume _returnvalue_2))
    (SaveGame|SaveGametoSlot _returnvalue "Options")
    (else
      (bind _returnvalue_3 (SaveGame|CreateSaveGameObject "/Game/GameModes/Saving/BP_AuroraSaveGame.BP_AuroraSaveGame_C"))
      (bind _asaurora_game_instance (Utilities|Casting|CastToAuroraGameInstance (Game|GetGameInstance)))
      (Variables|/Game/GameModes/Saving/BP_AuroraSaveGame.BP_AuroraSaveGame_C|SetScores _returnvalue_3 (Class|AuroraGameInstance|GetScores _asaurora_game_instance))
      (SaveGame|SaveGametoSlot _returnvalue_3 "Scores"))))