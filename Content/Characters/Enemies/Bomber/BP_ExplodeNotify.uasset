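; Animation notify for the Bomber enemy that applies its explosion damage to nearby enemies.
; On trigger, it finds the owner's sphere component tagged EXPLOSION and gets the BaseEnemy actors overlapping it.
; Each one's HealthComponent loses the BombEnemy owner's ExplosionDamage, then the animated mesh is hidden in game without affecting its children.
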(fn ReceivedNotify
  (params (MeshComp :type Skeletal%20Mesh%20Component%20Object%20Reference) (Animation :type Anim%20Sequence%20Base%20Object%20Reference))
  (bind _returnvalue (Components|GetOwner MeshComp))
  (for _array_element (Collision|GetOverlappingActors (Utilities|Array|Get(acopy) (Actor|GetComponentsbyTag _returnvalue "/Script/Engine.SphereComponent" "EXPLOSION")) "/Script/Aurora.BaseEnemy" :!class /Script/Engine.PrimitiveComponent)
    (bind _asbomb_enemy (Utilities|Casting|CastToBombEnemy _returnvalue))
    (Class|HealthComponent|DecreaseHealth (Actor|GetComponentbyClass _array_element "/Script/Aurora.HealthComponent") (Variables|/Script/Aurora.BombEnemy|GetExplosionDamage _asbomb_enemy)))
  (Development|SetHiddeninGame MeshComp true false)
  (return false))