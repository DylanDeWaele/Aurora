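; BP_Crystal_World is a player staff crystal that spins and visually shows the player's current ammo level.
; BeginPlay creates a dynamic material instance on the big crystal mesh.
; Each tick adds roughly one degree of world yaw, so spin speed depends on frame rate.
; Tick also casts the player character to BaseVRCharacter and drives the material's Mask Position from its scaled ammo percentage.
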(event EventBeginPlay
  (bind _returnvalue (Rendering|Material|CreateDynamicMaterialInstance (Variables|Default|GetSM_Crystal_Big) 0 0 "None" :!class /Script/Engine.PrimitiveComponent))
  (Variables|Default|SetMaterial _returnvalue))

(event Collision|EventActorBeginOverlap
  (params (OtherActor :type Actor%20Object%20Reference)))

(event EventTick
  (params (DeltaSeconds :type Float%20%28single-precision%29))
  (bind _sm_crystal_big (Variables|Default|GetSM_Crystal_Big))
  (bind _returnvalue (Transformation|GetWorldRotation _sm_crystal_big))
  (bind (_roll _pitch _yaw) (Math|Rotator|BreakRotator _returnvalue))
  (bind _result (Math|Float|IncrementFloat DeltaSeconds)
    (:%20%20
      (Transformation|SetWorldRotation (Variables|Default|GetSM_Crystal_Big) (Math|Rotator|MakeRotator _roll _pitch (+ (* _result 1.0) _yaw)) false false)
      (bind _asbase_vrcharacter (Utilities|Casting|CastToBaseVRCharacter (Game|GetPlayerCharacter 0)))
      (Rendering|Material|SetScalarParameterValue (Variables|Default|GetMaterial) "Mask Position" (* (Class|BaseVRCharacter|GetCurrentAmmoPercentage _asbase_vrcharacter) 6.0) :!class /Script/Engine.MaterialInstanceDynamic))))

(fn ConstructionScript)